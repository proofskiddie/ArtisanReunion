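; Tiger player character that runs automatically along world negative Y, with jumping and a draining stamina meter.
; Tick applies the constant movement input and lowers stamina over time, while BeginPlay adds a StaminaBar widget to the viewport.
; A counter limits jump presses to MaxJumps for double jumping and resets on landing.
; The zero-stamina check and capsule hit event have no behavior attached.
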(event OnComponentHit(CapsuleComponent)
  (params (HitComponent :type Primitive%20Component%20Object%20Reference) (OtherActor :type Actor%20Object%20Reference) (OtherComp :type Primitive%20Component%20Object%20Reference) (NormalImpulse :type Vector :default "0, 0, 0") (Hit :type Hit%20Result%20Structure%20%28by%20ref%29)))

(event EventBeginPlay
  (bind _returnvalue (UserInterface|CreateWidget "/Game/Kami_Game_Map/Blueprints/staminaBar.staminaBar_C"))
  (UserInterface|Viewport|AddtoViewport _returnvalue 0))

(event EventTick
  (params (DeltaSeconds :type Float%20%28single-precision%29))
  (Pawn|Input|AddMovementInput "0,-0.500000, 0" 5.0 false)
  (bind _output_get (Variables|Default|SetCurrentStamina (- (Variables|Default|GetCurrentStamina) (* DeltaSeconds 3.0))))
  (if (Math|Float|NearlyEqual(Float) _output_get 0.0 1e-06)
    _))

(event EventOnLanded
  (params (Hit :type Hit%20Result%20Structure%20%28by%20ref%29))
  ;[1 1 1] Double Jump
  (Variables|Default|SetJump%20Counter 0))

(event Input|ActionEvents|InputActionJump
  (params (Key :type Key%20Structure))
  ;[1 1 1] Double Jump
  (:Pressed
    (if (< (Variables|Default|GetJump%20Counter) (Variables|Default|GetMaxJumps))
      (Variables|Default|SetJump%20Counter (+ (Variables|Default|GetJump%20Counter) 1))
      (Character|Jump)))
  (:Released
    (Character|StopJumping)))

(fn ConstructionScript)